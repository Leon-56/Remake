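; Player-controlled ship pawn that moves in three axes and tests whether its pose completes a two-piece combination.
; Axis inputs drive movement, with forward and right rotated 90 degrees and height clamped between floor and ceiling.
; Each Tick compares a hard-coded transform and the ship's against a Solutions table row, using relative location and per-piece rotation tolerances.
; The result is only printed for debugging, and mouse yaw is disabled.
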(event EventBeginPlay)

(event Collision|EventActorBeginOverlap
  (params (OtherActor :type Actor%20Object%20Reference)))

(event EventTick
  (params (DeltaSeconds :type Float%20%28single-precision%29))
  (bind _returnvalue (Utilities|GetDataTableRow "/Game/02_Blueprint/Solutions.Solutions" "1")
    (:then
      (bind _iscombined (CallFunction|CheckCombination (Math|Transform|MakeTransform (+ "0.000000,0.000000,150.000000" "67.000000,0.000000,20.000000") "0,0.000000, 0") (Transformation|GetActorTransform) (.MeshTransform1 (Utilities|Struct|BreakSimpleSolution _returnvalue)) (.MeshTransform2 (Utilities|Struct|BreakSimpleSolution _returnvalue))))
      (Development|PrintString (Utilities|String|ToString(Boolean) _iscombined)))))

(event Input|AxisEvents|InputAxisMoveRight
  (params (AxisValue :type Float%20%28single-precision%29))
  (Pawn|Input|AddMovementInput (Math|Vector|RotateVector (Transformation|GetActorRightVector) "0,-90.000000, 0") AxisValue false))

(event Input|AxisEvents|InputAxisMoveUp
  (params (AxisValue :type Float%20%28single-precision%29))
  (bind _returnvalue (Transformation|GetActorLocation))
  (bind (_x _y _z) (Math|Vector|BreakVector _returnvalue))
  (bind _returnvalue_2 (Math|Float|Truncate _z))
  (if (< _returnvalue_2 500)
    (if (> _returnvalue_2 0)
      _
      (else
        (Transformation|SetActorLocation (Math|Vector|MakeVector _x _y 0.0) false false)))
    (else
      (Transformation|SetActorLocation (Math|Vector|MakeVector _x _y 5e+02) false false)))
  (Pawn|Input|AddMovementInput (Transformation|GetActorUpVector) AxisValue false))

(event Input|AxisEvents|InputAxisMoveForward
  (params (AxisValue :type Float%20%28single-precision%29))
  (Pawn|Input|AddMovementInput (Math|Vector|RotateVector (Transformation|GetActorForwardVector) "0,-90.000000, 0") AxisValue false))

(event Input|MouseEvents|MouseX
  (params (AxisValue :type Float%20%28single-precision%29))
  (if (not true)
    (Pawn|Input|AddControllerYawInput AxisValue)))

(event Input|MouseEvents|LeftMouseButton
  (params (Key :type Key%20Structure :default "None"))
  (:Pressed
    (Variables|Default|SetleftPressed true))
  (:Released
    (Variables|Default|SetleftPressed false)))

(fn ConstructionScript)

(fn IsCombined
  (params (LocationDifference :type Float%20%28single-precision%29) (RotationDifference1 :type Float%20%28single-precision%29) (RotationDifference2 :type Float%20%28single-precision%29))
  (return (and (< LocationDifference 15.0) (< (+ RotationDifference1 RotationDifference2) 1e+01))))

(fn CheckCombination
  (params (PlayerTransform1 :type Transform) (PlayerTransform2 :type Transform) (SolutionTransform1 :type Transform) (SolotionTransform2 :type Transform))
  (bind (_location _rotation) (Math|Transform|BreakTransform SolotionTransform2))
  (bind (_location_2 _rotation_2) (Math|Transform|BreakTransform PlayerTransform1))
  (bind (_location_3 _rotation_3) (Math|Transform|BreakTransform PlayerTransform2))
  (bind (_location_4 _rotation_4) (Math|Transform|BreakTransform SolutionTransform1))
  (bind (_roll _pitch _yaw) (Math|Rotator|BreakRotator _rotation))
  (bind (_roll_2 _pitch_2 _yaw_2) (Math|Rotator|BreakRotator _rotation_4))
  (bind (_roll_3 _pitch_3 _yaw_3) (Math|Rotator|BreakRotator _rotation_2))
  (bind (_roll_4 _pitch_4 _yaw_4) (Math|Rotator|BreakRotator _rotation_3))
  (bind _returnvalue (- _location_4 _location))
  (bind _returnvalue_2 (- _location_2 _location_3))
  (bind _returnvalue_3 (Math|Vector|MakeVector _roll_3 _pitch_3 _yaw_3))
  (bind _returnvalue_4 (Math|Vector|MakeVector _roll_4 _pitch_4 _yaw_4))
  (bind _returnvalue_5 (Math|Vector|MakeVector _roll_2 _pitch_2 _yaw_2))
  (bind _returnvalue_6 (Math|Vector|MakeVector _roll _pitch _yaw))
  (bind _returnvalue_7 (- _returnvalue_2 _returnvalue))
  (bind _returnvalue_8 (- _returnvalue_4 _returnvalue_6))
  (bind _returnvalue_9 (- _returnvalue_3 _returnvalue_5))
  (bind _returnvalue_10 (Math|Vector|VectorLength _returnvalue_7))
  (bind _returnvalue_11 (Math|Vector|VectorLength _returnvalue_8))
  (bind _returnvalue_12 (Math|Vector|VectorLength _returnvalue_9))
  (Development|PrintString (Utilities|String|Append "LocationDifference:" (Utilities|String|ToString(Float) _returnvalue_10)))
  (Development|PrintString (Utilities|String|Append "RotationDifference1:" (Utilities|String|ToString(Float) _returnvalue_12)))
  (Development|PrintString (Utilities|String|Append "RotationDifference2:" (Utilities|String|ToString(Float) _returnvalue_11)))
  (bind _biscombinationcompleted (CallFunction|IsCombined _returnvalue_10 _returnvalue_12 _returnvalue_11))
  (return _biscombinationcompleted))